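; Level manager Blueprint that initializes the level and reports when the game is over.
; The construction script calls InitLevel to set up the level.
; Tick watches IsGameOver and prints a restart message once, using a MessageSent flag that BeginPlay clears, though no restart logic follows the message.
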(event `self.ReceiveBeginPlay`
  (set `self.Message Sent` false))

(event `self.ReceiveTick`
  (params (DeltaSeconds :type "Float (single-precision)"))
  (if (and (`self.isGameOver`) (not (`self.Message Sent`)))
    (`KismetSystemLibrary.PrintString` "Restarting...")
    (set `self.Message Sent` true)))

(fn `UserConstructionScript`
  (`self.InitLevel`))