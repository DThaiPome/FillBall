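; Actor component that makes its owner tangible only when the game's active color matches its ObjectColor.
; On BeginPlay it binds to the ColorSwitchingBP game mode's color change and applies the material color.
; Each change swaps ColorMesh, assignable through SetColorMesh, between two material instances, re-tints it and toggles owner collision.
; ChangeMaterialOpacity is an alternative using a dynamic Opacity parameter, not called within this component.
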(event `Change Material Opacity`
  (params (Color :type "ObjectColor Enum" :default "RED"))
  (bind _returnvalue (`self.GetOwner`))
  (bind _returnvalue_2 (== Color (`self.objectColor`)))
  (if _returnvalue_2
    (set `self.Opacity` 1.0)
    (else
      (set `self.Opacity` 0.0)))
  (`Actor.SetActorEnableCollision` _returnvalue _returnvalue_2)
  (bind _asmaterial_instance_dynamic (cast `MaterialInstanceDynamic` (`PrimitiveComponent.GetMaterial` (`Actor.GetComponentByClass` _returnvalue "/Script/Engine.StaticMeshComponent") 0)))
  (`MaterialInstanceDynamic.SetScalarParameterValue` _asmaterial_instance_dynamic "Opacity" (`self.Opacity`)))

(event `self.ReceiveBeginPlay`
  (`|ExecutionSequence`
    (:`then_0`
      (bind _ascolor_switching_bp (cast `/Game/Blueprints/GameModes/ColorSwitchingBP` (`GameplayStatics.GetGameMode`)))
      (add `ColorSwitching.OnColorChange` _ascolor_switching_bp (delegate `On Color Changed`)))
    (:`then_1`
      (`self.UpdateMaterialColor` "Color"))))

(event `On Color Changed`
  (params (color :type "ObjectColor Enum" :default "RED"))
  (`self.Change Material` color))

(event `Change Material`
  (params (Color :type "ObjectColor Enum" :default "RED"))
  (bind _objectcolor (`self.objectColor`))
  (bind _color_mesh (`self.Color Mesh`))
  (bind _returnvalue (== Color _objectcolor))
  (if _returnvalue
    (`PrimitiveComponent.SetMaterial` _color_mesh 0 "/Game/Materials/ColorActorMaterial_O_Inst1.ColorActorMaterial_O_Inst1")
    (else
      (`PrimitiveComponent.SetMaterial` _color_mesh 0 "/Game/Materials/ColorActorMaterial_Inst1.ColorActorMaterial_Inst1")))
  (`ColorSwitching.UpdateMaterialColor` _color_mesh _objectcolor "Color")
  (`Actor.SetActorEnableCollision` (`self.GetOwner`) _returnvalue)
  (`KismetSystemLibrary.PrintString` "Hello"))

(event `Set Color Mesh`
  (params (`Color Mesh` :type "StaticMeshComponent Object Reference"))
  (set `self.Color Mesh` `Color Mesh`))