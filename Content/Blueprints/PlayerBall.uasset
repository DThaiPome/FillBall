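; Player-controlled physics ball pawn that rolls through a level and loses on overlapping a KillFloor-tagged actor.
; Yaw-relative input drives force on the ground and torque in the air, with ground contact set by Hit and cleared each Tick.
; Mouse input rotates the controller with clamped pitch.
; The LevelManager game mode receives the loss, and its game-over flag makes Tick reload the level after a delay.
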(event `InputAxis|MoveRight`
  (params (AxisValue :type "Float (single-precision)"))
  (bind _returnvalue (`KismetMathLibrary.MakeRotator` 0.0 0.0 (.yaw (`self.GetControlRotation`))))
  ;[1 1 1] Calculate movement  input for ball
  (set `self.MoveDirection` (+ (* (`KismetMathLibrary.GetRightVector` _returnvalue) AxisValue) (* (`KismetMathLibrary.GetForwardVector` _returnvalue) (stale `InputAxis|MoveForward` AxisValue))) :!label _label))

(event `InputAxis|MouseX`
  (params (AxisValue :type "Float (single-precision)"))
  ;[1 1 1] Calculate camera rotation values
  (set `self.LookVector` (* (`KismetMathLibrary.MakeVector2D` AxisValue (* (stale `InputAxis|MouseY` AxisValue) -1.0)) (`self.MouseSensitivity`)) :!label _label_2))

(event `self.ReceiveActorBeginOverlap`
  (params (OtherActor :type "Actor Object Reference"))
  ;[1 1 1] Lose when you fall off
  (if (`ActorComponent.ComponentHasTag` (`Actor.RootComponent` OtherActor) "KillFloor")
    (bind _aslevel_manager (cast `LevelManager` (`GameplayStatics.GetGameMode`)))
    (`LevelManager.LevelLost` _aslevel_manager)))

(event `InputAxis|MouseY`
  (params (AxisValue :type "Float (single-precision)"))
  ;[1 1 1] Calculate camera rotation values
  (goto _label_2))

(event `InputAxis|MoveForward`
  (params (AxisValue :type "Float (single-precision)"))
  ;[1 1 1] Calculate movement  input for ball
  (goto _label))

(event `self.ReceiveTick`
  (params (DeltaSeconds :type "Float (single-precision)"))
  ;[1 1 1] OnTick Behaviour
  (bind _aslevel_manager (cast `LevelManager` (`GameplayStatics.GetGameMode`)))
  (if (`LevelManager.isGameOver` _aslevel_manager)
    (`self.Restart Level` (`self.Level Restart Delay`))
    (else
      (`|ExecutionSequence`
        (:`then_0`
          (if (`self.On Ground`)
            (`self.Move Ball` DeltaSeconds)
            (else
              (`self.Spin Ball` DeltaSeconds))))
        (:`then_1`
          (`self.Rotate Camera` DeltaSeconds))
        (:`then_2`
          (set `self.On Ground` false))))))

(event `Move Ball`
  (params (`Delta Seconds` :type "Float (double-precision)"))
  ;[1 1 1] Move the ball
  (`PrimitiveComponent.AddForce` (`self.Ball`) (* (* (`self.MoveDirection`) `Delta Seconds`) (`self.Speed`)) "None" true))

(event `Spin Ball`
  (params (`Delta Seconds` :type "Float (double-precision)"))
  ;[1 1 1] Rotate the ball when it's in the air
  (`PrimitiveComponent.AddTorqueInDegrees` (`self.Ball`) (* (`KismetMathLibrary.MakeVector` (* (.y (* (* (`self.MoveDirection`) `Delta Seconds`) (`self.Aerial Rotate Speed`))) -1.0) (.x (* (* (`self.MoveDirection`) `Delta Seconds`) (`self.Aerial Rotate Speed`)))) 1.0) "None" true))

(event `Rotate Camera`
  (params (`Delta Seconds` :type "Float (double-precision)"))
  (bind (_x _y) (`KismetMathLibrary.BreakVector2D` (* (`self.LookVector`) `Delta Seconds`)))
  (bind _returnvalue (`KismetMathLibrary.FClamp` (+ _y (`self.Current Pitch`)) (`self.Min Camera Pitch`) (`self.Max Camera Pitch`)))
  ;[1 1 1] Rotate Camera
  (`|ExecutionSequence`
    (:`then_0`
      (`self.AddControllerYawInput` _x))
    (:`then_1`
      (set `self.Current Pitch` _returnvalue))
    (:`then_2`
      (`Controller.SetControlRotation` (`self.GetController`) (`KismetMathLibrary.MakeRotator` (.roll (`self.GetControlRotation`)) _returnvalue (.yaw (`self.GetControlRotation`)))))))

(event `self.ReceiveBeginPlay`
  ;[1 1 1] Initialize Pitch Variable
  (set `self.Current Pitch` (.pitch (`self.GetControlRotation`))))

(event `self.ReceiveHit`
  (params (MyComp :type "PrimitiveComponent Object Reference") (Other :type "Actor Object Reference") (OtherComp :type "PrimitiveComponent Object Reference") (bSelfMoved :type Boolean) (HitLocation :type "Vector Structure") (HitNormal :type "Vector Structure") (NormalImpulse :type "Vector Structure") (Hit :type "HitResult Structure (by ref)"))
  ;[1 1 1] Detect if the ball is on the ground
  (set `self.On Ground` true))

(event `Restart Level`
  (params (Delay :type "Float (double-precision)"))
  ;[1 1 1] Restart the current level
  (`KismetSystemLibrary.Delay` Delay)
  (bind _returnvalue (`GameplayStatics.GetCurrentLevelName` true))
  (`GameplayStatics.OpenLevel` (`KismetStringLibrary.Conv_StringToName` _returnvalue)))

(fn `UserConstructionScript`)