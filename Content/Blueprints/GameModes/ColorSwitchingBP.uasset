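; Game mode for a color-switching game that manages streamed levels, per-level timer and pickup count, and music.
; BeginPlay loads the current level; each load resets stats, sets the color to red, enables game input and recomputes current and next levels from the level list.
; Winning shows the end-level UI with UI-only input, while restart and next-level events request streamed level changes.
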(event `Set Control`
  (params (`In Level` :type Boolean))
  (bind _returnvalue (`GameplayStatics.GetPlayerController` 0))
  (if `In Level`
    (`WidgetBlueprintLibrary.SetInputMode_GameOnly` _returnvalue)
    (else
      (`WidgetBlueprintLibrary.SetInputMode_UIOnlyEx` _returnvalue null)))
  (set `PlayerController.bShowMouseCursor` (not `In Level`) _returnvalue))

(event `Signal Level Loaded`
  (params (`Loaded Level` :type Name))
  (`self.SignalLevelLoaded` `Loaded Level`))

(event `self.ReceiveBeginPlay`
  (add `self.OnLevelLoaded` (delegate `Level Start`))
  (`KismetSystemLibrary.Delay` 0.2)
  (`self.Set Levels`)
  (`self.RequestLoadStreamLevel` (`self.Current Level`))
  (`GameplayStatics.PlaySound2D` "/Game/Sounds/EverJustRefuseToSlepMan_Cue.EverJustRefuseToSlepMan_Cue" 1.0 1.0 0.0 null null))

(event `Level Start` :!signature `self.OnLevelLoaded`
  (params (loadedLevelName :type Name))
  (`|ExecutionSequence`
    (:`then_0`
      (set `self.PickupsCollected` 0)
      (set `self.Timer` 0.0))
    (:`then_1`
      (`self.ChangeColor` "RED"))
    (:`then_2`
      (add `self.OnGameOver` (delegate `On Game Over`)))
    (:`then_3`
      (`self.Set Control` true))
    (:`then_4`
      (`self.Set Levels`))))

(event `Show End UI`
  (bind _returnvalue (`|CreateWidget` "/Game/Blueprints/UI/EndLevelUI.EndLevelUI_C"))
  (`UserWidget.AddToViewport` _returnvalue 0)
  (`self.Set Control` false))

(event `Restart Level`
  (`self.RequestChangeStreamLevel` (`self.Current Level`) (`self.Current Level`)))

(event `To Next Level`
  (`self.RequestChangeStreamLevel` (`self.Current Level`) (`self.Next Level`)))

(event `On Game Over` :!signature `self.OnGameOver`
  (params (levelWon :type Boolean))
  (if levelWon
    (`self.Show End UI`)))

(event `self.ReceiveTick`
  (params (DeltaSeconds :type "Float (single-precision)"))
  (if (not (`self.isGameOver`))
    (set `self.Timer` (+ DeltaSeconds (`self.Timer`)))))

(event `Set Levels`
  (bind _levels (`self.Levels`))
  (bind _returnvalue (`self.GetNextLevel` _levels (`self.End Level`) (`self.Current Level`)))
  (bind _output_get (set `self.Next Level` _returnvalue))
  (set `self.Current Level` (`|GetArrayItem` _levels (mod (- (`KismetArrayLibrary.Array_Find` _levels _output_get) 1) (`KismetArrayLibrary.Array_Length` _levels)))))

(event `PickupCollected`
  (`/Engine/EditorBlueprintResources/StandardMacros.IncrementInt` (`self.PickupsCollected`)))

(fn `UserConstructionScript`)