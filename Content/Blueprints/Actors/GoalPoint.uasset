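; GoalPoint is a level goal actor that wins the level when the player's pawn overlaps it.
; On overlap it spawns a GoalParticleBurst at its Sphere component's world transform and destroys itself.
; The same sequence then casts the game mode to LevelManager and calls LevelWon, so the game mode handles the win.
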(event `self.ReceiveActorBeginOverlap`
  (params (OtherActor :type "Actor Object Reference"))
  (if (== OtherActor (`GameplayStatics.GetPlayerPawn` 0))
    (`|ExecutionSequence`
      (:`then_0`
        (`|SpawnActorFromClass` "/Game/Blueprints/Actors/GoalParticleBurst.GoalParticleBurst_C" (`SceneComponent.GetSocketTransform` (`self.Sphere`) "None" "RTS_World") "Undefined" "OverrideRootScale" null null)
        (`self.K2_DestroyActor`))
      (:`then_1`
        (bind _aslevel_manager (cast `LevelManager` (`GameplayStatics.GetGameMode`)))
        (`LevelManager.LevelWon` _aslevel_manager)))))

(fn `UserConstructionScript`)