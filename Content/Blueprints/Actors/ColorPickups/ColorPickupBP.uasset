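; ColorPickupBP is a colored pickup actor that changes the game's active color when the player touches it.
; On begin play it updates its material to match its Color.
; On overlap with an actor whose root component is tagged Player, it runs its pickup handling, then passes Color to the ColorSwitchingBP game mode and notifies it that a pickup was collected.
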(event `self.ReceiveBeginPlay`
  (`self.UpdateMaterialColor` "Color"))

(event `self.ReceiveActorBeginOverlap`
  (params (OtherActor :type "Actor Object Reference"))
  ;[1 1 1] Deactivate and change color on contact with player
  (if (`ActorComponent.ComponentHasTag` (`Actor.RootComponent` OtherActor) "Player")
    (`|ExecutionSequence`
      (:`then_0`
        (`self.OnPickup`))
      (:`then_1`
        (bind _ascolor_switching_bp (cast `/Game/Blueprints/GameModes/ColorSwitchingBP` (`GameplayStatics.GetGameMode`)))
        (`ColorSwitching.ChangeColor` _ascolor_switching_bp (`self.color`)))
      (:`then_2`
        (`/Game/Blueprints/GameModes/ColorSwitchingBP.PickupCollected` _ascolor_switching_bp)))))

(fn `UserConstructionScript`)